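; Base gravity bridge actor, built around a Cylinder and two end spheres, that supplies the point on its axis level with the player.
; GetAxis finds the first world axis on which SphereL and SphereR differ, then combines the player's coordinate on that axis with the Cylinder's other two.
; It assumes an axis-aligned bridge and does not clamp the point between the spheres.
; The event graph holds only disabled default events.
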(fn `getAxis`
  (returns (Output_Get :type "Vector Structure"))
  (bind (_returnvalue_x _returnvalue_y _returnvalue_z) (`KismetMathLibrary.BreakVector` (`SceneComponent.K2_GetComponentLocation` (`self.Cylinder`))))
  (bind (_returnvalue_x_2 _returnvalue_y_2 _returnvalue_z_2) (`KismetMathLibrary.BreakVector` (`SceneComponent.K2_GetComponentLocation` (`self.SphereL`))))
  (bind (_returnvalue_x_3 _returnvalue_y_3 _returnvalue_z_3) (`KismetMathLibrary.BreakVector` (`self.K2_GetActorLocation` (`GameplayStatics.GetPlayerCharacter` 0))))
  (bind (_returnvalue_x_4 _returnvalue_y_4 _returnvalue_z_4) (`KismetMathLibrary.BreakVector` (`SceneComponent.K2_GetComponentLocation` (`self.SphereR`))))
  (if (not (`KismetMathLibrary.NearlyEqual_FloatFloat` _returnvalue_x_2 _returnvalue_x_4 1.0))
    (set `self.AxisVector` (`KismetMathLibrary.MakeVector` _returnvalue_x_3 _returnvalue_y _returnvalue_z))
    (return (`self.AxisVector`))
    (elif (not (`KismetMathLibrary.NearlyEqual_FloatFloat` _returnvalue_y_2 _returnvalue_y_4 1.0))
      (set `self.AxisVector` (`KismetMathLibrary.MakeVector` _returnvalue_x _returnvalue_y_3 _returnvalue_z))
      (return (`self.AxisVector`))
      (elif (not (`KismetMathLibrary.NearlyEqual_FloatFloat` _returnvalue_z_2 _returnvalue_z_4 1.0))
        (set `self.AxisVector` (`KismetMathLibrary.MakeVector` _returnvalue_x _returnvalue_y _returnvalue_z_3))
        (return (`self.AxisVector`))))))

(fn `UserConstructionScript`
  (`parent.UserConstructionScript`))